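; BP_Door is a two-panel sliding door that opens and closes through its OpenDoor event.
; BeginPlay caches both panels' relative start locations, and the DoorMovement timeline lerps them in opposite directions along MoveDirection.
; Opening plays the timeline with an attached slide sound, while closing reverses it from its current position without triggering a sound.
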(event `self.ReceiveBeginPlay`
  (set `self.DoorLeftStart` (`SceneComponent.RelativeLocation` (`self.Door 1`)))
  (set `self.DoorRightStart` (`SceneComponent.RelativeLocation` (`self.Door 2`))))

(event `OpenDoor`
  (params (Open :type Boolean))
  (bind _doorleftstart (`self.DoorLeftStart`))
  (bind _doorrightstart (`self.DoorRightStart`))
  (if Open
    (`GameplayStatics.SpawnSoundAttached` "/Game/Audio/SFX/SFX_Obj_SLideDoorOpen.SFX_Obj_SLideDoorOpen" (`self.Scene`) "None" (0.0 0.0 0.0) (struct) "KeepRelativeOffset" false 1.0 1.0 0.0 null null)
    (bind (_direction _newtrack_0) (`Timeline|DoorMovement` :!label _label)
      (:`Update`
        (`SceneComponent.K2_SetRelativeLocation` (`self.Door 1`) (`KismetMathLibrary.VLerp` _doorleftstart (+ _doorleftstart (`self.Move Direction`)) _newtrack_0) false false)
        (`SceneComponent.K2_SetRelativeLocation` (`self.Door 2`) (`KismetMathLibrary.VLerp` _doorrightstart (- _doorrightstart (`self.Move Direction`)) _newtrack_0) false false)))
    (else
      (goto _label :!via `Reverse`))))

(fn `UserConstructionScript`)