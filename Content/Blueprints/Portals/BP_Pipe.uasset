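; BP_Pipe is a portal pipe that teleports any actor overlapping its Box to a linked pipe and rescales it.
; Overlap plays an entry sound and waits a second, then moves the actor to OtherPipe's local SpawnPoint converted to world space.
; The actor's new scale is this pipe's scale times NewScale.
; The exit sound also plays at this pipe, and the teleport result is printed for debugging.
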(event `self.Box.OnComponentBeginOverlap`
  (params (OverlappedComponent :type "PrimitiveComponent Object Reference") (OtherActor :type "Actor Object Reference") (OtherComp :type "PrimitiveComponent Object Reference") (OtherBodyIndex :type Integer) (bFromSweep :type Boolean) (SweepResult :type "HitResult Structure (by ref)"))
  (bind _returnvalue (`self.K2_GetActorLocation`))
  (bind _otherpipe (`self.OtherPipe`))
  (`GameplayStatics.PlaySoundAtLocation` "/Game/Audio/SFXs/SFX_PipeIn.SFX_PipeIn" _returnvalue (struct) 1.0 1.0 0.0 null null null null)
  (`KismetSystemLibrary.Delay` 1.0)
  (bind (_sweephitresult _returnvalue_2) (`self.K2_SetActorLocation` OtherActor (`KismetMathLibrary.TransformLocation` (`self.GetTransform` _otherpipe) (`/Game/Blueprints/Portals/BP_Pipe.SpawnPoint` _otherpipe)) false true))
  (`self.SetActorScale3D` OtherActor (* (`self.GetActorScale3D`) (`self.NewScale`)))
  (`GameplayStatics.PlaySoundAtLocation` "/Game/Audio/SFXs/SFX_PipeOut.SFX_PipeOut" _returnvalue (struct) 1.0 1.0 0.0 null null null null)
  (`KismetSystemLibrary.PrintString` (`KismetStringLibrary.Conv_BoolToString` _returnvalue_2)))

(fn `UserConstructionScript`)