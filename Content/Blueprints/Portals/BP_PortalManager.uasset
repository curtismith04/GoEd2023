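; Portal manager that drives the view components of a linked Source and Target portal pair from the player's camera.
; While Active, each Tick moves both PortalViews to the camera position plus the same Source-minus-Target plane offset.
; Source's view rotation derives from camera rotation relative to Target and vice versa, with that actor's yaw added back.
; An alternative relative-rotation and debug-line approach remains disconnected.
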(event `self.ReceiveTick`
  (params (DeltaSeconds :type "Float (single-precision)"))
  (bind _returnvalue (`self.K2_GetActorRotation` (`self.Source`)))
  (bind _returnvalue_2 (`self.K2_GetActorRotation` (`self.Target`)))
  (bind _transformcomponent (`PlayerCameraManager.TransformComponent` (`PlayerController.PlayerCameraManager` (`GameplayStatics.GetPlayerController` 0))))
  (bind _transformcomponent_2 (`PlayerCameraManager.TransformComponent` (`PlayerController.PlayerCameraManager` (`GameplayStatics.GetPlayerController` 0))))
  (bind (_returnvalue_roll _returnvalue_pitch _returnvalue_yaw) (`KismetMathLibrary.BreakRotator` (`KismetMathLibrary.NormalizedDeltaRotator` (`SceneComponent.K2_GetComponentRotation` _transformcomponent) _returnvalue)))
  (bind (_returnvalue_roll_2 _returnvalue_pitch_2 _returnvalue_yaw_2) (`KismetMathLibrary.BreakRotator` (`KismetMathLibrary.NormalizedDeltaRotator` (`SceneComponent.K2_GetComponentRotation` _transformcomponent_2) _returnvalue_2)))
  (if (`self.Active`)
    (`SceneComponent.K2_SetWorldLocationAndRotation` (`Portal.PortalView` (`self.Source`)) (+ (`SceneComponent.K2_GetComponentLocation` _transformcomponent_2) (- (`SceneComponent.K2_GetComponentLocation` (`Portal.Plane` (`self.Source`))) (`SceneComponent.K2_GetComponentLocation` (`Portal.Plane` (`self.Target`))))) (`KismetMathLibrary.MakeRotator` _returnvalue_roll_2 _returnvalue_pitch_2 (+ _returnvalue_yaw_2 (.yaw _returnvalue_2))) false false)
    (`SceneComponent.K2_SetWorldLocationAndRotation` (`Portal.PortalView` (`self.Target`)) (+ (`SceneComponent.K2_GetComponentLocation` _transformcomponent) (- (`SceneComponent.K2_GetComponentLocation` (`Portal.Plane` (`self.Source`))) (`SceneComponent.K2_GetComponentLocation` (`Portal.Plane` (`self.Target`))))) (`KismetMathLibrary.MakeRotator` _returnvalue_roll _returnvalue_pitch (+ _returnvalue_yaw (.yaw _returnvalue))) false false)))

(fn `UserConstructionScript`)