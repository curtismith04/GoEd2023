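; B_Spinner is a marble-triggered spinner that rotates its MainShelf when an actor tagged "Marble" overlaps its W component.
; The overlap also plays a fanfare and fires the RotateOtherSpinner dispatcher, which a spinner binds to on its LinkedRotator at BeginPlay.
; Both triggers share a DoOnce with no reset, so the MoveRotator timeline runs only once.
; Each timeline update adds the lerped yaw as a delta, so rotation accumulates.
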(event `self.ReceiveBeginPlay`
  (bind _linkedrotator (`self.LinkedRotator`)
    (:`then`
      (add `self.RotateOtherSpinner` _linkedrotator (delegate `RotateOtherSpinner_Event`)))
    (:`else`)))

(event `RotateOtherSpinner_Event`
  (`self.RotateSpinner`))

(event `RotateSpinner`
  (`/Engine/EditorBlueprintResources/StandardMacros.DoOnce` false :!label _label
    (:`Completed`
      (bind (_direction _rotate) (`Timeline|MoveRotator` :!via `PlayFromStart`)
        (:`Update`
          (`SceneComponent.K2_AddRelativeRotation` (`self.MainShelf`) (`KismetMathLibrary.MakeRotator` 0.0 0.0 (`KismetMathLibrary.Lerp` 0.0 (`self.RotAmnt`) _rotate)) false false))))))

(event `self.w.OnComponentBeginOverlap`
  (params (OverlappedComponent :type "PrimitiveComponent Object Reference") (OtherActor :type "Actor Object Reference") (OtherComp :type "PrimitiveComponent Object Reference") (OtherBodyIndex :type Integer) (bFromSweep :type Boolean) (SweepResult :type "HitResult Structure (by ref)"))
  (if (`self.ActorHasTag` OtherActor "Marble")
    (`self.RotateOtherSpinner`)
    (`GameplayStatics.PlaySound2D` "/Game/Audio/SFXs/SFX_Fanfare.SFX_Fanfare" 1.0 1.0 0.0 null null)
    (goto _label)))

(fn `UserConstructionScript`)