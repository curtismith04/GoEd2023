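; BP_Door1 is a door that swings open when a marble lands on its linked Switch.
; It binds to the Switch's marble-landed dispatcher on BeginPlay, then plays a sound and uses a timeline to yaw the Door mesh to a quarter turn.
; When the timeline finishes, it fires its door-open dispatcher and unhides an optional FinalSwitch actor.
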(event `self.ReceiveBeginPlay`
  (bind _switch (`self.Switch`)
    (:`then`
      (add `/Game/Blueprints/Portals/BP_MarbleSwitch.ED_MarbleLanded` _switch (delegate `ED_MarbleLanded_Event`)))
    (:`else`)))

(event `ED_MarbleLanded_Event`
  (`self.OpenDoor`))

(event `OpenDoor`
  (`GameplayStatics.PlaySoundAtLocation` "/Game/Audio/SFXs/SFX_DoorOpen.SFX_DoorOpen" (`SceneComponent.K2_GetComponentLocation` (`self.Door`)) (struct) 1.0 1.0 0.0 null null null null)
  (bind (_direction _doorrotation) (`Timeline|DoorOpen` :!via `PlayFromStart`)
    (:`Update`
      (`SceneComponent.K2_SetRelativeRotation` (`self.Door`) (`KismetMathLibrary.MakeRotator` 0.0 0.0 (`KismetMathLibrary.Lerp` 0.0 90.0 _doorrotation)) false false))
    (:`Finished`
      (`self.ED_DoorOpen`)
      (bind _finalswitch (`self.FinalSwitch`)
        (:`then`
          (`self.SetActorHiddenInGame` _finalswitch false))
        (:`else`)))))

(fn `UserConstructionScript`)