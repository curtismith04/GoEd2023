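; BP_MarbleSwitch is a one-shot switch triggered when an actor tagged "Marble" overlaps its capsule.
; Triggering broadcasts a marble-landed event, changes the cube's material, plays a fanfare and opens the linked DoorToOpen.
; With DisableCol set, the capsule starts without collision until DoorEnablingCol's door-open dispatcher re-enables it, allowing switches to be gated by doors.
; When IsCongrats is set, it also pushes a congratulations UI prompt and spawns two confetti effects.
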(event `self.ReceiveBeginPlay`
  (if (`self.DisableCol`)
    (`PrimitiveComponent.SetCollisionEnabled` (`self.Capsule`) "NoCollision")
    (bind _doorenablingcol (`self.DoorEnablingCol`)
      (:`then`
        (add `/Game/Blueprints/Portals/BP_Door1.ED_DoorOpen` _doorenablingcol (delegate `ED_DoorOpen_Event`)))
      (:`else`))))

(event `ED_DoorOpen_Event`
  (`PrimitiveComponent.SetCollisionEnabled` (`self.Capsule`) "QueryAndProbe"))

(event `self.Capsule.OnComponentBeginOverlap`
  (params (OverlappedComponent :type "PrimitiveComponent Object Reference") (OtherActor :type "Actor Object Reference") (OtherComp :type "PrimitiveComponent Object Reference") (OtherBodyIndex :type Integer) (bFromSweep :type Boolean) (SweepResult :type "HitResult Structure (by ref)"))
  (bind _returnvalue (`self.K2_GetActorLocation`))
  (if (`self.ActorHasTag` OtherActor "Marble")
    (`/Engine/EditorBlueprintResources/StandardMacros.DoOnce` false
      (:`Completed`
        (`self.ED_MarbleLanded`)
        (`PrimitiveComponent.SetMaterial` (`self.Cube`) 0 "/Game/ArtAssets/Materials/MI_PlasticSwitch.MI_PlasticSwitch")
        (`GameplayStatics.PlaySound2D` "/Game/Audio/SFXs/SFX_Fanfare.SFX_Fanfare" 1.0 1.0 0.0 null null)
        (bind _doortoopen (`self.DoorToOpen`)
          (:`then`
            (`/Game/Blueprints/Portals/BP_Door1.OpenDoor` _doortoopen))
          (:`else`
            _))
        (if (`self.isCongrats`)
          (bind _asbp_first_person_player_controller (cast `/Game/FirstPerson/Blueprints/BP_FirstPersonPlayerController` (`GameplayStatics.GetPlayerController` 0)))
          (`/Game/UI/Widgets/W_CUI_Base.PushCongratsPrompt` (`/Game/FirstPerson/Blueprints/BP_FirstPersonPlayerController.UI_Base` _asbp_first_person_player_controller))
          (`NiagaraFunctionLibrary.SpawnSystemAttached` "/Game/VFXs/NS_Confetti.NS_Confetti" null "None" (- _returnvalue (0.0 50.0 0.0)) (struct) "KeepRelativeOffset")
          (`NiagaraFunctionLibrary.SpawnSystemAttached` "/Game/VFXs/NS_Confetti.NS_Confetti" null "None" (+ _returnvalue (0.0 50.0 0.0)) (struct) "KeepRelativeOffset"))))))

(fn `UserConstructionScript`)