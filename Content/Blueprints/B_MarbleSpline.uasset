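; B_MarbleSpline carries an overlapping marble along a spline by snapping it to a MarbleMover component.
; MoveAlongSpline, not called within this graph, starts a looping timer that advances the mover by distance and spawns an attached rising-tunnel sound.
; The first found B_Marble overlapping a "Gap" actor pauses the timer and sound.
; A DockedPipe event from any B_Floatable resumes both.
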(event `self.ReceiveBeginPlay`
  (bind _outactors (`GameplayStatics.GetAllActorsOfClass` "/Game/Blueprints/B_Marble.B_Marble_C"))
  ;[1 1 1] This is used to watch for when the marble comes to a gap stop. It just stops the marble movement on the spline
  (add `self.OnActorBeginOverlap` (`|GetArrayItem` _outactors) (delegate `OnActorBeginOverlap_Event`))
  (bind _outactors_2 (`GameplayStatics.GetAllActorsOfClass` "/Game/Blueprints/Portals/B_Floatable.B_Floatable_C"))
  (for _array_element _outactors_2
    (add `/Game/Blueprints/Portals/B_Floatable.DockedPipe` _array_element (delegate `DockedPipe_Event`))))

(event `OnActorBeginOverlap_Event` :!signature `self.OnActorBeginOverlap`
  (params (OverlappedActor :type "Actor Object Reference") (OtherActor :type "Actor Object Reference"))
  (bind _timermarblemover (`self.TimerMarbleMover`))
  ;[1 1 1] This is used to watch for when the marble comes to a gap stop. It just stops the marble movement on the spline
  (if (`self.ActorHasTag` OtherActor "Gap")
    (if (`KismetSystemLibrary.K2_IsTimerActiveHandle` _timermarblemover)
      (`KismetSystemLibrary.K2_PauseTimerHandle` _timermarblemover)
      (bind _risersfx (`self.RiserSFX`)
        (:`then`
          (`AudioParameterControllerInterface.SetTriggerParameter` _risersfx "Pause"))
        (:`else`)))))

(event `DockedPipe_Event`
  (bind _timermarblemover (`self.TimerMarbleMover`))
  (if (`KismetSystemLibrary.K2_IsTimerPausedHandle` _timermarblemover)
    (`KismetSystemLibrary.K2_UnPauseTimerHandle` _timermarblemover)
    (bind _risersfx (`self.RiserSFX`)
      (:`then`
        (`AudioParameterControllerInterface.SetTriggerParameter` _risersfx "Resume"))
      (:`else`))))

(event `MoveAlongSpline`
  (bind _returnvalue (`KismetSystemLibrary.K2_SetTimerDelegate` (delegate `MoveMarble`) (`self.Time`) true))
  (set `self.TimerMarbleMover` _returnvalue)
  (bind _returnvalue_2 (`GameplayStatics.SpawnSoundAttached` "/Game/Audio/SFXs/SFX_MarbleRisingUpTunnel.SFX_MarbleRisingUpTunnel" (`self.MarbleMover`) "None" (0.0 0.0 0.0) (struct) "KeepRelativeOffset" false 1.0 1.0 0.0 null null))
  (set `self.RiserSFX` _returnvalue_2))

(event `MoveMarble`
  (bind _marblemover (`self.MarbleMover`))
  (bind _output_get (set `self.DistanceAlongSpline` (+ (* (`self.Time`) (`self.SplineSpeed`)) (`self.DistanceAlongSpline`))))
  (bind (_returnvalue_location _returnvalue_rotation) (`KismetMathLibrary.BreakTransform` (`SplineComponent.GetTransformAtDistanceAlongSpline` (`self.Spline`) _output_get "Local" false)))
  (`SceneComponent.K2_SetRelativeTransform` _marblemover (`KismetMathLibrary.MakeTransform` _returnvalue_location _returnvalue_rotation (`SceneComponent.RelativeScale3D` _marblemover)) false false))

(event `self.ReceiveActorBeginOverlap`
  (params (OtherActor :type "Actor Object Reference"))
  (if (`self.ActorHasTag` OtherActor "Marble")
    (`self.K2_AttachToComponent` OtherActor (`self.MarbleMover`) "None" "SnapToTarget" "SnapToTarget" "KeepRelative" true)))

(fn `UserConstructionScript`)