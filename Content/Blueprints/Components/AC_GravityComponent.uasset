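; AC_GravityComponent is a component that switches a static mesh between engine gravity and a custom directional gravity.
; On BeginPlay it applies the starting state through ToggleGravity, which only takes effect while the mesh simulates physics.
; While engine gravity is off, Tick pushes the mesh along GravityDirection with a force scaled by GravityScale and mass, divided by delta time.
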(event `self.ReceiveBeginPlay`
  (`self.Toggle Gravity` (`self.StartWithGravity`)))

(event `self.ReceiveTick`
  (params (DeltaSeconds :type "Float (single-precision)"))
  (bind _staticmesh (`self.StaticMesh`))
  (if (not (`self.isGravityOn`))
    (`PrimitiveComponent.AddForce` _staticmesh (/ (* (* (`self.Gravity Direction`) (`self.Gravity Scale`)) (`PrimitiveComponent.GetMass` _staticmesh)) DeltaSeconds) "None" false)))

(fn `Toggle Gravity`
  (params (`Gravity On` :type Boolean))
  (bind _staticmesh (`self.StaticMesh`))
  (if (`SceneComponent.IsSimulatingPhysics` (`self.StaticMesh`) "None")
    (if `Gravity On`
      (`PrimitiveComponent.SetEnableGravity` _staticmesh true)
      (set `self.isGravityOn` true)
      (else
        (`PrimitiveComponent.SetEnableGravity` _staticmesh false)
        (set `self.isGravityOn` false)))))