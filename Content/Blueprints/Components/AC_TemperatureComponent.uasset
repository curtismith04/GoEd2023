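; Actor component that tracks a temperature value, rising or falling between zero and MaxTemp.
; ChangeTemp clears the current timer and starts a looping one that calls IncreaseTemp or DecreaseTemp, depending on the Hot flag.
; Each tick steps the value, heating slightly faster than cooling, then clamps at the limit and stops the timer.
; Both step functions print the current temperature to screen, and the event graph is unused.
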(fn `ChangeTemp`
  (params (Hot :type Boolean))
  (`KismetSystemLibrary.K2_ClearAndInvalidateTimerHandle` (`self.TempTimer`))
  (if Hot
    (bind _returnvalue (`KismetSystemLibrary.K2_SetTimer` null "IncreaseTemp" 0.05 true))
    (set `self.TempTimer` _returnvalue)
    (else
      (bind _returnvalue_2 (`KismetSystemLibrary.K2_SetTimer` null "DecreaseTemp" 0.05 true))
      (set `self.TempTimer` _returnvalue_2))))

(fn `DecreaseTemp`
  (bind _returnvalue (- (`self.CurrentTemp`) 0.4))
  (`KismetSystemLibrary.PrintString` (`KismetStringLibrary.Conv_DoubleToString` (`self.CurrentTemp`)))
  (if (< _returnvalue 0.0)
    (set `self.CurrentTemp` 0.0)
    (`KismetSystemLibrary.K2_ClearAndInvalidateTimerHandle` (`self.TempTimer`))
    (else
      (set `self.CurrentTemp` _returnvalue))))

(fn `IncreaseTemp`
  (bind _returnvalue (+ (`self.CurrentTemp`) 0.5))
  (`KismetSystemLibrary.PrintString` (`KismetStringLibrary.Conv_DoubleToString` (`self.CurrentTemp`)))
  (if (> _returnvalue (`self.MaxTemp`))
    (set `self.CurrentTemp` (`self.MaxTemp`))
    (`KismetSystemLibrary.K2_ClearAndInvalidateTimerHandle` (`self.TempTimer`))
    (else
      (set `self.CurrentTemp` _returnvalue))))