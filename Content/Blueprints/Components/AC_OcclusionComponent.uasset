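; Actor component that reports when its owning actor comes into view or stops being rendered, through the OnObjectInView and OnObjectOccluded dispatchers.
; Each tick it checks WasRecentlyRendered on the owner, using the frame's delta time as tolerance.
; The in-view event fires once after a short continuous time on screen, while the occluded event fires on the first unrendered tick after that.
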(event `self.ReceiveTick`
  (params (DeltaSeconds :type "Float (single-precision)"))
  (if (`Actor.WasRecentlyRendered` (`self.GetOwner`) DeltaSeconds)
    (bind _output_get (set `self.TimeInView` (+ (`self.TimeInView`) DeltaSeconds)))
    (if (and (not (`self.ShouldChange`)) (> _output_get 0.2))
      (set `self.ShouldChange` true)
      (`self.OnObject In View`))
    (else
      (set `self.TimeInView` 0.0)
      (if (`self.ShouldChange`)
        (set `self.ShouldChange` false)
        (`self.OnObjectOccluded`)))))