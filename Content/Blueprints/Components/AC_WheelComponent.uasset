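; Actor component that spins a mesh like a wheel and lets hit results add to its speed.
; Tick rotates the mesh by Speed, then decays it per frame, by a fixed step when positive and by Friction when negative, with clamping.
; AddWheelSpeed adds Acceleration if LockDirection is set, otherwise derives a signed, clamped push from hit height and trace direction against the owner's forward vector.
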(event `self.ReceiveTick`
  (params (DeltaSeconds :type "Float (single-precision)"))
  (bind _friction (`self.Friction`))
  (bind _speed (`self.Speed`))
  (if (!= _speed 0.0)
    (`SceneComponent.K2_AddLocalRotation` (`self.Mesh`) (* (`self.Rotation Axis`) (* _speed DeltaSeconds)) false false)
    (`/Engine/EditorBlueprintResources/StandardMacros.CompareFloat` (`self.Speed`)
      (:`>`
        (set `self.Speed` (`KismetMathLibrary.FClamp` (- (`self.Speed`) 1.0) 0.0 (`self.MaxVelocity`))))
      (:`<`
        (set `self.Speed` (`KismetMathLibrary.FClamp` (+ (`self.Speed`) _friction) (* (`self.MaxVelocity`) (* _friction -1.0)) 0.0))))))

(event `Add Wheel Speed`
  (params (`Hit Result` :type "HitResult Structure (by ref)"))
  (bind (_bblockinghit _binitialoverlap _time _distance _location _impactpoint _normal _impactnormal _physmat _hitactor _hitcomponent _hitbonename _bonename _hititem _elementindex _faceindex _tracestart _traceend) (`GameplayStatics.BreakHitResult` `Hit Result`))
  (bind _acceleration (`self.Acceleration`))
  (bind (_returnvalue_x _returnvalue_y _returnvalue_z) (`KismetMathLibrary.BreakVector` (- (`SceneComponent.K2_GetComponentLocation` _hitcomponent) _location)))
  (if (`self.LockDirection`)
    (set `self.Speed` (+ (`self.Speed`) (`self.Acceleration`)))
    (else
      (set `self.Speed` (+ (`self.Speed`) (`KismetMathLibrary.FClamp` (* (* _returnvalue_z (`KismetMathLibrary.Dot_VectorVector` (`KismetMathLibrary.Normal` (- _tracestart _traceend)) (`Actor.GetActorForwardVector` (`self.GetOwner`)))) -1.0) (* _acceleration -1.0) _acceleration))))))

(fn `GetSpeed`
  (returns (Speed :type "Float (double-precision)"))
  (return (`self.Speed`)))