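; BP_QuarkSlot is an interactable socket actor that accepts one quark of a matching type from the interacting character.
; On interact, PlaceQuark searches the character's held quarks, removes the first match, snaps it to the slot's sphere, makes it visible and resets its effect to the base system.
; A successful placement locks the slot, stops the sphere responding to visibility traces and notifies the GI_EMJ23 game instance.
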(event `/Game/Blueprints/Interfaces/Interactable.Interact`
  (params (Character :type "/Game/Blueprints/BP_PlayerCharacter Object Reference") (Component :type "PrimitiveComponent Object Reference"))
  (bind _placed (`self.Place Quark` Character))
  (if _placed
    (`PrimitiveComponent.SetCollisionResponseToChannel` (`self.Sphere`) "ECC_Visibility" "ECR_Ignore")
    (`/Game/GameItems/GI_EMJ23.QuarkPlaced` (cast `/Game/GameItems/GI_EMJ23` (`GameplayStatics.GetGameInstance`) :!pure true))))

(fn `Place Quark`
  (params (Character :type "/Game/Blueprints/BP_PlayerCharacter Object Reference"))
  (returns (Placed :type Boolean))
  (locals (QuarkActor :type "/Game/Assets/FPWeapon/Projectiles/BP_Projectile Object Reference"))
  (bind _quarkactor (`local.QuarkActor`))
  (bind _quarkactor_2 (`local.QuarkActor`))
  (if (not (`self.QuarkPlaced`))
    (for _array_element (`/Game/Blueprints/BP_PlayerCharacter.HeldQuarks` Character)
      (if (`|EnumEquality` (`/Game/Assets/FPWeapon/Projectiles/BP_Projectile.QuarkType` _array_element) (`self.Quark`))
        (bind _output_get (set `local.QuarkActor` _array_element))
        (`/Game/Blueprints/BP_PlayerCharacter.RemoveQuark` (`local.Character`) _output_get)
        (`SceneComponent.SetVisibility` (`/Game/Assets/FPWeapon/Projectiles/BP_Projectile.Quark Body` _quarkactor) true false)
        (`self.K2_AttachToComponent` _quarkactor (`self.Sphere`) "None" "SnapToTarget" "SnapToTarget" "KeepWorld" true)
        (`NiagaraComponent.SetAsset` (`/Game/Assets/FPWeapon/Projectiles/BP_Projectile.Quark Body` _quarkactor_2) (`/Game/Assets/FPWeapon/Projectiles/BP_Projectile.Base Quark System` _quarkactor_2) true)
        (set `self.QuarkPlaced` true)
        (return true)))
    (return false)))

(fn `UserConstructionScript`)