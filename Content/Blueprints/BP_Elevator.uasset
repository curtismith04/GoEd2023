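; BP_Elevator is an elevator actor that moves between its start location and a Direction offset, driven by a wheel that reacts to water hits.
; WaterEvent passes each hit to ACWheelComponent to add wheel speed, and the construction script assigns the Cylinder as that component's mesh.
; While the wheel speed is nonzero, Tick advances a clamped alpha by wheel speed divided by Speed and lerps the actor's position without sweeping.
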(event `self.ReceiveBeginPlay`
  (bind _output_get (set `self.StartLocation` (`self.K2_GetActorLocation`)))
  (set `self.Relative End Location` (+ _output_get (`self.Direction`))))

(event `self.ReceiveTick`
  (params (DeltaSeconds :type "Float (single-precision)"))
  (bind _speed (`/Game/Blueprints/Components/AC_WheelComponent.GetSpeed` (`self.AC_WheelComponent`)))
  (if (!= _speed 0.0)
    (set `self.Alpha` (`KismetMathLibrary.FClamp` (+ (`self.Alpha`) (* DeltaSeconds (/ _speed (`self.Speed`))))))
    (`self.K2_SetActorLocation` (`KismetMathLibrary.VLerp` (`self.StartLocation`) (`self.Relative End Location`) (`self.Alpha`)))))

(event `/Game/Blueprints/Interfaces/Water.Water Event`
  (params (Component :type "PrimitiveComponent Object Reference") (Hit :type "HitResult Structure"))
  (`/Game/Blueprints/Components/AC_WheelComponent.Add Wheel Speed` (`self.AC_WheelComponent`) Hit))

(fn `UserConstructionScript`
  (set `/Game/Blueprints/Components/AC_WheelComponent.Mesh` (`self.Cylinder`) (`self.AC_WheelComponent`)))