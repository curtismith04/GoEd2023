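; BP_Fireball is a projectile that sets burnable targets alight on contact.
; On BeginPlay it scales its Velocity variable by the ProjectileMovement component's initial speed to launch itself.
; A Sphere overlap calls Burn through the Burnable interface when the component has the "Burnable" tag and its actor implements that interface.
; The fireball destroys itself on any Sphere overlap, burnable or not.
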(event `self.ReceiveBeginPlay`
  (bind _projectilemovement (`self.ProjectileMovement`))
  (set `MovementComponent.Velocity` (* (`self.Velocity`) (`ProjectileMovementComponent.InitialSpeed` _projectilemovement)) _projectilemovement))

(event `self.Sphere.OnComponentBeginOverlap`
  (params (OverlappedComponent :type "PrimitiveComponent Object Reference") (OtherActor :type "Actor Object Reference") (OtherComp :type "PrimitiveComponent Object Reference") (OtherBodyIndex :type Integer) (bFromSweep :type Boolean) (SweepResult :type "HitResult Structure (by ref)"))
  (if (and (`ActorComponent.ComponentHasTag` OtherComp "Burnable") (`KismetSystemLibrary.DoesImplementInterface` OtherActor "/Game/Blueprints/Interfaces/Burnable.Burnable_C"))
    (`/Game/Blueprints/Interfaces/Burnable.Burn` (cast `/Game/Blueprints/Interfaces/Burnable` OtherActor :!pure true)))
  (`self.K2_DestroyActor`))

(fn `UserConstructionScript`)