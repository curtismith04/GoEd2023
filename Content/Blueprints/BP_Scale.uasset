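; Balance-scale puzzle actor that drives a linked door by comparing the masses of two cylinders.
; Each water event adds mass to Cylinder, and interacting empties a bucket by resetting the hit component to Cylinder's starting mass.
; Both actions pass a near-equal mass check to the door, if one is valid.
; With a door, water events also start a one-time jingle and feed it Cylinder's mass as a parameter.
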(event `self.ReceiveBeginPlay`
  (set `self.Base Mass` (`PrimitiveComponent.GetMass` (`self.Cylinder`))))

(event `/Game/Blueprints/Interfaces/Water.Water Event`
  (params (Component :type "PrimitiveComponent Object Reference") (Hit :type "HitResult Structure"))
  (bind _cylinder (`self.Cylinder`))
  (bind _sfx_obj_scale_jingle (`self.SFX_Obj_Scale_Jingle`))
  (bind _returnvalue (`PrimitiveComponent.GetMass` _cylinder))
  (`PrimitiveComponent.SetMassOverrideInKg` _cylinder "None" (+ _returnvalue 1.0) true)
  (`/Engine/EditorBlueprintResources/StandardMacros.IsValid` (`self.Door`)
    (:`Is Valid`
      (`self.Try Door`)
      (`|ExecutionSequence`
        (:`then_0`
          (`/Engine/EditorBlueprintResources/StandardMacros.DoOnce` false
            (:`Completed`
              (`ActorComponent.Activate` _sfx_obj_scale_jingle false))))
        (:`then_1`
          (`AudioParameterControllerInterface.SetFloatParameter` _sfx_obj_scale_jingle "Mass" _returnvalue))))))

(event `/Game/Blueprints/Interfaces/Interactable.Interact`
  (params (Character :type "/Game/Blueprints/BP_PlayerCharacter Object Reference") (Component :type "PrimitiveComponent Object Reference"))
  ;[1 1 1] Empty Bucket
  (`PrimitiveComponent.SetMassOverrideInKg` (cast `StaticMeshComponent` Component :!pure true) "None" (`self.Base Mass`) true)
  (`/Engine/EditorBlueprintResources/StandardMacros.IsValid` (`self.Door`)
    (:`Is Valid`
      (`self.Try Door`))))

(fn `Try Door`
  (`/Game/Blueprints/BP_Door.OpenDoor` (`self.Door`) (`KismetMathLibrary.NearlyEqual_FloatFloat` (`PrimitiveComponent.GetMass` (`self.Cylinder`)) (`PrimitiveComponent.GetMass` (`self.Cylinder1`)) 5.0)))

(fn `UserConstructionScript`)