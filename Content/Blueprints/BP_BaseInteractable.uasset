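; BP_BaseInteractable is a base interactable that shows and hides an interaction prompt through the player's UI.
; On BeginPlay it caches UIBase from BP_PlayerCharacter, retrying each tick until both the character and a valid UI exist.
; The Display event pushes a prompt with the interact text and modal border style, or removes it, using a displayed flag to avoid duplicate pushes.
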(event `self.ReceiveBeginPlay`
  (bind _asbp_player_character (cast `/Game/Blueprints/BP_PlayerCharacter` (`GameplayStatics.GetPlayerCharacter` 0) :!label _label)
    (:`then`
      (bind _ui_base (`/Game/Blueprints/BP_PlayerCharacter.UI_Base` _asbp_player_character)
        (:`then`
          (set `self.UI Base` _ui_base))
        (:`else`
          (`KismetSystemLibrary.DelayUntilNextTick` :!label _label_2)
          (goto _label))))
    (:`CastFailed`
      (goto _label_2))))

(event `/Game/Blueprints/Interfaces/Interactable.Display`
  (params (`Should Display` :type Boolean))
  (if `Should Display`
    (if (not (`self.isWidgetDisplayed`))
      (bind _ui_base (`self.UI Base`)
        (:`then`
          (`/Game/UI/Widgets/W_CUI_Base.PushPrompt` _ui_base (`self.Interact Text`) "/Game/UI/Styles/CUIStyle_Border_Modal_Interact.CUIStyle_Border_Modal_Interact_C" (`|ConvertAsset` _ui_base) 0)
          (set `self.isWidgetDisplayed` true))
        (:`else`)))
    (else
      ;[0.4791 0.3001 1] Closing of the prompt is handled on it's own
      (bind _ui_base_2 (`self.UI Base`)
        (:`then`
          (`/Game/UI/Widgets/W_CUI_Base.RemovePromopt` _ui_base_2)
          (set `self.isWidgetDisplayed` false))
        (:`else`)))))

(fn `UserConstructionScript`)