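; B_Interactable is a poster that reveals a hint when the player uses the grab input nearby.
; The construction script applies the hidden material, and a Box overlap with Player-tagged actors toggles the E-key hint image and an in-range flag.
; Grabbing in range swaps to the shown material once, hides the prompt and destroys the Box.
; BeginPlay caches UIBase from the first-person controller, though these graphs never use it.
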(event `self.ReceiveBeginPlay`
  (bind _asbp_first_person_player_controller (cast `/Game/FirstPerson/Blueprints/BP_FirstPersonPlayerController` (`GameplayStatics.GetPlayerController` 0)))
  (set `self.UI Base` (`/Game/FirstPerson/Blueprints/BP_FirstPersonPlayerController.UI_Base` _asbp_first_person_player_controller)))

(event `self.Box.OnComponentBeginOverlap`
  (params (OverlappedComponent :type "PrimitiveComponent Object Reference") (OtherActor :type "Actor Object Reference") (OtherComp :type "PrimitiveComponent Object Reference") (OtherBodyIndex :type Integer) (bFromSweep :type Boolean) (SweepResult :type "HitResult Structure (by ref)"))
  (if (`self.ActorHasTag` OtherActor "Player")
    (`SceneComponent.SetVisibility` (`self.EHintImage`) true false)
    (set `self.InRange` true)))

(event `self.Box.OnComponentEndOverlap`
  (params (OverlappedComponent :type "PrimitiveComponent Object Reference") (OtherActor :type "Actor Object Reference") (OtherComp :type "PrimitiveComponent Object Reference") (OtherBodyIndex :type Integer))
  (if (`self.ActorHasTag` OtherActor "Player")
    (`SceneComponent.SetVisibility` (`self.EHintImage`) false false)
    (set `self.InRange` false)))

(event `EnhancedInput|/Game/FirstPerson/Input/Actions/IA_Grab`
  (params (ActionValue :type Boolean) (ElapsedSeconds :type "Float (double-precision)") (TriggeredSeconds :type "Float (double-precision)") (InputAction :type "InputAction Object Reference" :default "/Game/FirstPerson/Input/Actions/IA_Grab.IA_Grab"))
  (:`Triggered`
    (if (`self.InRange`)
      (`/Engine/EditorBlueprintResources/StandardMacros.DoOnce` false
        (:`Completed`
          (`PrimitiveComponent.SetMaterial` (`self.Poster`) 0 (`self.ShownHint`))
          (`SceneComponent.SetVisibility` (`self.EHintImage`) false false)
          (`ActorComponent.K2_DestroyComponent` (`self.Box`)))))))

(fn `UserConstructionScript`
  (`PrimitiveComponent.SetMaterial` (`self.Poster`) 0 (`self.HiddenHint`)))