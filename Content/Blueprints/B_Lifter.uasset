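; B_Lifter is a lift actor that rises and opens two doors when a marble lands on its linked switch.
; On BeginPlay it binds to the switch's marble-landed dispatcher, which plays a timeline.
; Each update adds scaled timeline movement to the Cube's current height, while a DoOnce opens BigDoor and SmallDoor on the first update.
; A debug key also plays the timeline; the LifterLooper timer event is empty.
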(event Custom|ED_MarbleLanded_Event
  (bind _self self)
  (bind _cube (Variables|Default|GetCube _self))
  (bind _returnvalue (Transformation|GetWorldLocation _cube))
  (bind _movement (Timeline|Timeline PlayFromStart)
    (:Update
      (Transformation|SetActorTransform _self (Math|Transform|MakeTransform (Math|Vector|MakeVector (.x _returnvalue) (.y _returnvalue) (+ (* _movement 2.0) (.z _returnvalue))) (Transformation|GetActorRotation _self) (Transformation|GetActorScale3D _self)))
      (Utilities|FlowControl|DoOnce false
        (:Completed
          (Default|OpenDoor (Variables|Default|GetBigDoor)))))))

(event Custom|LifterLooper)

(event EventBeginPlay
  (bind _switchreference (Variables|Default|GetSwitchReference)
    (:then
      (EventDispatchers|AssignEDMarbleLanded _switchreference (delegate Custom|ED_MarbleLanded_Event))
      (Utilities|Time|SetTimerbyEvent (delegate Custom|LifterLooper) 0.0))
    (:else)))

(event Input|KeyboardEvents|DebugKey1
  (params (Key :type Key%20Structure :default "None") (ActionValue :type Input%20Action%20Value%20Structure))
  (bind _self self)
  (bind _cube (Variables|Default|GetCube _self))
  (bind _returnvalue (Transformation|GetWorldLocation _cube))
  (:Pressed
    (bind _movement (Timeline|Timeline PlayFromStart)
      (:Update
        (Transformation|SetActorTransform _self (Math|Transform|MakeTransform (Math|Vector|MakeVector (.x _returnvalue) (.y _returnvalue) (+ (* _movement 2.0) (.z _returnvalue))) (Transformation|GetActorRotation _self) (Transformation|GetActorScale3D _self)))
        (Utilities|FlowControl|DoOnce false
          (:Completed
            (Default|OpenDoor (Variables|Default|GetBigDoor))))))))

(fn ConstructionScript)