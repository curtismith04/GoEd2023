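; BP_Torch is a torch actor that can be lit or extinguished and spreads fire to burnable objects.
; A "Burning" tag on its Sphere marks the lit state, alongside Niagara flames and a point light.
; While burning, sphere overlaps with "Burnable"-tagged components call Burn through the Burnable interface.
; Burn and Extinguish toggle that state and broadcast TorchStatusChanged; StartLit false puts it out at BeginPlay.
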(event `self.ReceiveBeginPlay`
  (`parent.ReceiveBeginPlay`)
  (if (not (`self.StartLit`))
    (`self.PutOutTorch`)
    (`AudioComponent.Stop` (`self.SFX_Obj_Torch`))
    (`GameplayStatics.SpawnSoundAttached` "/Game/Audio/SFX/SFX_Obj_Torch_Extinguish.SFX_Obj_Torch_Extinguish" (`self.StaticMesh`) "None" (0.0 0.0 0.0) (struct) "KeepRelativeOffset" false 1.0 1.0 0.0 null null)))

(event `self.Sphere.OnComponentBeginOverlap`
  (params (OverlappedComponent :type "PrimitiveComponent Object Reference") (OtherActor :type "Actor Object Reference") (OtherComp :type "PrimitiveComponent Object Reference") (OtherBodyIndex :type Integer) (bFromSweep :type Boolean) (SweepResult :type "HitResult Structure (by ref)"))
  (`/Engine/EditorBlueprintResources/StandardMacros.IsValid` OtherComp
    (:`Is Valid`
      (if (and (`ActorComponent.ComponentHasTag` OverlappedComponent "Burning") (`ActorComponent.ComponentHasTag` OtherComp "Burnable"))
        (`/Game/Blueprints/Interfaces/Burnable.Burn` (cast `/Game/Blueprints/Interfaces/Burnable` OtherActor :!pure true))))))

(event `/Game/Blueprints/Interfaces/Burnable.Burn`
  (`self.Try Light Torch`)
  (`self.TorchStatusChanged` self true))

(event `/Game/Blueprints/Interfaces/Burnable.Extinguish`
  (`self.PutOutTorch`)
  (`self.TorchStatusChanged` self))

(fn `PutOutTorch`
  (`ActorComponent.Deactivate` (`self.Niagara`))
  (`KismetArrayLibrary.Array_RemoveItem` (`ActorComponent.ComponentTags` (`self.Sphere`)) "Burning")
  (`SceneComponent.SetVisibility` (`self.PointLight`) false false))

(fn `Try Light Torch`
  (if (not (`ActorComponent.ComponentHasTag` (`self.Sphere`) "Burning"))
    (`ActorComponent.Activate` (`self.Niagara`) false)
    (`SceneComponent.SetVisibility` (`self.PointLight`) true false)
    (`KismetArrayLibrary.Array_Add` (`ActorComponent.ComponentTags` (`self.Sphere`)) "Burning")))

(fn `UserConstructionScript`
  (`parent.UserConstructionScript`))