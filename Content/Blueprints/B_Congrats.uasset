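; B_Congrats is a trigger actor that celebrates when an actor tagged Player overlaps its Box.
; A two-pass loop spawns NS_Confetti attached to its root, using the player mesh's world location and a point offset along X as relative offsets.
; The loop body continues into a one-second Delay, then pushes the congrats prompt through the first-person player controller's UIBase.
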(event `self.Box.OnComponentBeginOverlap`
  (params (OverlappedComponent :type "PrimitiveComponent Object Reference") (OtherActor :type "Actor Object Reference") (OtherComp :type "PrimitiveComponent Object Reference") (OtherBodyIndex :type Integer) (bFromSweep :type Boolean) (SweepResult :type "HitResult Structure (by ref)"))
  (bind _returnvalue (`SceneComponent.K2_GetComponentLocation` (`Character.Mesh` (`GameplayStatics.GetPlayerCharacter` 0))))
  (if (`self.ActorHasTag` OtherActor "Player")
    (for _index (range 2)
      (`NiagaraFunctionLibrary.SpawnSystemAttached` "/Game/VFXs/NS_Confetti.NS_Confetti" (`self.DefaultSceneRoot`) "None" (select `int` _index :`0` _returnvalue :`1` (+ _returnvalue (500.0 0.0 0.0))) (struct) "KeepRelativeOffset")
      (`KismetSystemLibrary.Delay` 1.0)
      (bind _asbp_first_person_player_controller (cast `/Game/FirstPerson/Blueprints/BP_FirstPersonPlayerController` (`GameplayStatics.GetPlayerController` 0)))
      (`/Game/UI/Widgets/W_CUI_Base.PushCongratsPrompt` (`/Game/FirstPerson/Blueprints/BP_FirstPersonPlayerController.UI_Base` _asbp_first_person_player_controller)))))

(fn `UserConstructionScript`)