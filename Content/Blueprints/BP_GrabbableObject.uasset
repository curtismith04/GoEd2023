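; Grabbable interactable actor that a character picks up and drops through its physics handle.
; Interact toggles the grab on the static mesh, pauses the character's tracing while held and calls Display(false) on pickup.
; On BeginPlay, objects flagged as gravity puzzle balls deactivate their gravity component.
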(event `self.ReceiveBeginPlay`
  (`parent.ReceiveBeginPlay`)
  (if (`self.isGravityPuzzleBall`)
    (`ActorComponent.Deactivate` (`self.AC_GravityComponent`))))

(event `/Game/Blueprints/Interfaces/Interactable.Interact`
  (params (Character :type "/Game/Blueprints/BP_PlayerCharacter Object Reference") (Component :type "PrimitiveComponent Object Reference"))
  ;[1 1 1] Physics Handle Grabbing
  (if (`self.isGrabbed`)
    (`PhysicsHandleComponent.ReleaseComponent` (`/Game/Blueprints/BP_PlayerCharacter.PhysicsHandle` Character))
    (set `self.isGrabbed` false)
    (set `/Game/Blueprints/BP_PlayerCharacter.ShouldTrace` true Character)
    (else
      (set `/Game/Blueprints/BP_PlayerCharacter.ShouldTrace` false Character)
      (`PhysicsHandleComponent.GrabComponentAtLocationWithRotation` :`self` (`/Game/Blueprints/BP_PlayerCharacter.PhysicsHandle` Character) :`Component` (`self.StaticMesh`) :`Location` (`self.K2_GetActorLocation`))
      (set `self.isGrabbed` true)
      (`/Game/Blueprints/Interfaces/Interactable.Display` false))))

(fn `UserConstructionScript`
  (`parent.UserConstructionScript`))