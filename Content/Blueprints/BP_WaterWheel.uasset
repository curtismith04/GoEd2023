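; BP_WaterWheel is a physics water wheel that gains speed from water events and drives its own audio.
; WaterEvent passes hits to ACWheelComponent, which is given the static mesh in the construction script.
; A looping 0.1-second timer maps the mesh's angular speed to an audio float parameter, though its name is left as None.
; Paired DoOnce gates fire the StartWheel and StopWheel audio triggers once per change between moving and still.
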(event `self.ReceiveBeginPlay`
  (`KismetSystemLibrary.K2_SetTimerDelegate` (delegate `05sLooper`) 0.1 true))

(event `05sLooper`
  (bind _audio (`self.Audio`))
  (bind _returnvalue (`KismetMathLibrary.VSize` (`PrimitiveComponent.GetPhysicsAngularVelocityInDegrees` (`self.StaticMesh`) "None")))
  (`AudioParameterControllerInterface.SetFloatParameter` (`self.Audio`) "None" (`KismetMathLibrary.MapRangeClamped` _returnvalue 0.0 500.0 0.0 1.0))
  (if (> _returnvalue 0.0)
    (`|ExecutionSequence`
      (:`then_0`
        (`/Engine/EditorBlueprintResources/StandardMacros.DoOnce` false :!label _label
          (:`Completed`
            (`AudioParameterControllerInterface.SetTriggerParameter` _audio "StartWheel"))))
      (:`then_1`
        (goto _label_2 :!via `Reset`)))
    (else
      (`|ExecutionSequence`
        (:`then_0`
          (goto _label :!via `Reset`))
        (:`then_1`
          (`/Engine/EditorBlueprintResources/StandardMacros.DoOnce` false :!label _label_2
            (:`Completed`
              (`AudioParameterControllerInterface.SetTriggerParameter` _audio "StopWheel"))))))))

(event `self.ReceiveTick`
  (params (DeltaSeconds :type "Float (single-precision)")))

(event `/Game/Blueprints/Interfaces/Water.Water Event`
  (params (Component :type "PrimitiveComponent Object Reference") (Hit :type "HitResult Structure"))
  (`/Game/Blueprints/Components/AC_WheelComponent.Add Wheel Speed` (`self.AC_WheelComponent`) Hit))

(fn `UserConstructionScript`
  (set `/Game/Blueprints/Components/AC_WheelComponent.Mesh` (`self.StaticMesh`) (`self.AC_WheelComponent`)))