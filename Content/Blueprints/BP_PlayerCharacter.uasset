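; First-person player character Blueprint with a quark gun, cycling quark inventory, physics-handle holding and UI prompts.
; Movement uses input vectors under gravity and camera-relative launches in zero G; shooting forwards to QuarkGun, and Tick keeps the handle target ahead of the camera.
; TraceForObjects toggles highlights on tagged Interactable actors.
; Gun spawning, trace timer startup and menu pushes sit in unreached chains.
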(event `self.ReceiveBeginPlay`
  (`self.UI_BeginPlay`)
  (`EnhancedInputSubsystemInterface.AddMappingContext` (pcsubsystem `EnhancedInputLocalPlayerSubsystem` (`GameplayStatics.GetPlayerController` 0)) null 0 (struct)))

(event `self.ReceiveTick`
  (params (DeltaSeconds :type "Float (single-precision)"))
  (bind _camera (`self.Camera`))
  (`PhysicsHandleComponent.SetTargetLocationAndRotation` (`self.PhysicsHandle`) (+ (`SceneComponent.K2_GetComponentLocation` _camera) (* (`SceneComponent.GetForwardVector` _camera) 200.0)) (`SceneComponent.K2_GetComponentRotation` (`self.Camera`))))

(event `EnhancedInput|/Game/FirstPerson/Input/Actions/IA_Move`
  (params (ActionValue :type "Vector2D Structure") (ElapsedSeconds :type "Float (double-precision)") (TriggeredSeconds :type "Float (double-precision)") (InputAction :type "InputAction Object Reference" :default "/Game/FirstPerson/Input/Actions/IA_Move.IA_Move"))
  (bind (_x _y) (`KismetMathLibrary.BreakVector2D` ActionValue))
  (bind (_x_2 _y_2) (`KismetMathLibrary.BreakVector2D` ActionValue))
  (bind _camera (`self.Camera`))
  (:`Triggered`
    (if (> (`CharacterMovementComponent.GravityScale` (`self.CharacterMovement`)) 0.0)
      (`PawnMovementComponent.AddInputVector` (`self.CharacterMovement`) (+ (* (`self.GetActorForwardVector`) _x_2) (* (`self.GetActorRightVector`) _y_2)) false)
      (else
        ;[1 1 1] Zero G
        (`self.LaunchCharacter` (* (+ (* (`SceneComponent.GetForwardVector` _camera) _x) (* (`SceneComponent.GetRightVector` _camera) _y)) 3.0))))))

(event `EnhancedInput|/Game/FirstPerson/Input/Actions/IA_Shoot`
  (params (ActionValue :type Boolean) (ElapsedSeconds :type "Float (double-precision)") (TriggeredSeconds :type "Float (double-precision)") (InputAction :type "InputAction Object Reference" :default "/Game/FirstPerson/Input/Actions/IA_Shoot.IA_Shoot"))
  (bind _quarkgun (`self.QuarkGun`))
  (:`Triggered`
    (`/Engine/EditorBlueprintResources/StandardMacros.IsValid` _quarkgun
      (:`Is Valid`
        (`/Game/Blueprints/BP_QuarkGun.PrimaryAction` _quarkgun ActionValue)))))

(event `UI_BeginPlay`
  ;[0.4791 0.3001 1] UI
  (bind _returnvalue (`|CreateWidget` "/Game/UI/Widgets/W_CUI_Base.W_CUI_Base_C" (`GameplayStatics.GetPlayerController` 0)))
  (bind _output_get (set `self.UI_Base` _returnvalue))
  (`UserWidget.AddToViewport` _output_get 0))

(event `PushPrompt`
  (params (TextToDisplay :type Text) (ImageStyle :type "CommonBorderStyle Class Reference") (PromptOwner :type "/Game/UI/Widgets/W_CUI_Base Soft Object Reference") (PromptIndex :type Integer))
  ;[0.4791 0.3001 1] UI
  (`/Game/UI/Widgets/W_CUI_Base.PushEForPrompt` (`self.UI_Base`) TextToDisplay ImageStyle PromptOwner PromptIndex))

(fn `ObtainQuark`
  (params (`New Quark` :type "/Game/Assets/FPWeapon/Projectiles/BP_Projectile Object Reference"))
  (`KismetArrayLibrary.Array_AddUnique` (`self.HeldQuarks`) `New Quark`)
  (`self.SwitchQuarks`)
  ;[1 1 1] Remove when new systems are active
  (`self.SetActorScale3D` `New Quark` (0.3 0.3 0.3)))

(fn `RemoveQuark`
  (params (Quark :type "/Game/Assets/FPWeapon/Projectiles/BP_Projectile Object Reference"))
  (bind _returnvalue (- (`KismetArrayLibrary.Array_Length` (`self.HeldQuarks`)) 1))
  (`|ExecutionSequence`
    (:`then_0`
      (if (== (`/Game/Blueprints/BP_QuarkGun.ActiveQuark` (`self.QuarkGun`)) Quark)
        (`self.SwitchQuarks`)))
    (:`then_1`
      (`KismetArrayLibrary.Array_RemoveItem` (`self.HeldQuarks`) Quark)
      (if (> (`self.QuarkIndex`) _returnvalue)
        (set `self.QuarkIndex` _returnvalue)))))

(fn `SwitchQuarks`
  (bind _quarkindex (`self.QuarkIndex`))
  (bind _output (`|GetArrayItem` (`self.HeldQuarks`) _quarkindex))
  (`SceneComponent.SetVisibility` (`/Game/Assets/FPWeapon/Projectiles/BP_Projectile.Quark Body` (`|GetArrayItem` (`self.HeldQuarks`) (`self.QuarkIndex`))) false false)
  (bind _result (`/Engine/EditorBlueprintResources/StandardMacros.IncrementInt` (`self.QuarkIndex`))
    (:`  `
      (if (> _result (- (`KismetArrayLibrary.Array_Length` (`self.HeldQuarks`)) 1))
        (set `self.QuarkIndex` 0))
      (`/Game/Blueprints/BP_QuarkGun.SetActiveQuark` (`self.QuarkGun`) _output)
      (`SceneComponent.SetVisibility` (`/Game/Assets/FPWeapon/Projectiles/BP_Projectile.Quark Body` _output) true false)
      (`self.ED_SwitchQuarks` _quarkindex _output))))

(fn `TraceForObjects`
  (bind _camera (`self.Camera`))
  (bind _viewedactor (`self.ViewedActor`))
  (bind _returnvalue (`SceneComponent.K2_GetComponentLocation` _camera))
  (if (`self.ShouldTrace`)
    (bind (_outhit _returnvalue_2) (`KismetSystemLibrary.LineTraceSingle` :`Start` _returnvalue :`End` (+ _returnvalue (* (`SceneComponent.GetForwardVector` _camera) (`self.LookDistance`))) :`TraceChannel` "TraceTypeQuery1" :`DrawTime` 0.5))
    (set `self.Hit Result` _outhit)
    (if _returnvalue_2
      (bind (_bblockinghit _binitialoverlap _time _distance _location _impactpoint _normal _impactnormal _physmat _hitactor _hitcomponent) (`GameplayStatics.BreakHitResult` _outhit))
      (if (and (`ActorComponent.ComponentHasTag` _hitcomponent "Interact") (`KismetSystemLibrary.DoesImplementInterface` _hitactor "/Game/Blueprints/Interfaces/Interactable.Interactable_C"))
        (bind _output_get (set `self.ViewedActor` _hitactor))
        (`/Game/Blueprints/Interfaces/Interactable.Display` (cast `/Game/Blueprints/Interfaces/Interactable` _output_get :!pure true) true)
        (else
          (`/Engine/EditorBlueprintResources/StandardMacros.IsValid` _viewedactor :!label _label
            (:`Is Valid`
              (bind _asinteractable (cast `/Game/Blueprints/Interfaces/Interactable` _viewedactor))
              (`/Game/Blueprints/Interfaces/Interactable.Display` _asinteractable false)
              (set `self.ViewedActor` null)))))
      (else
        (goto _label)))))

(fn `UserConstructionScript`)