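; Rail actor that lays spline mesh segments along its Spline component in the construction script, with no active runtime logic.
; It divides the spline into fixed-length steps scaled by actor Y scale, bending each Y-forward segment with start and end tangents clamped to segment length.
; Segments use query-and-probe collision.
; CreateSplineMesh duplicates this logic for a supplied spline, but returns after the first segment and is not called here.
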(fn `CreateSplineMesh`
  (params (CurrentSpline :type "SplineComponent Object Reference"))
  (bind (_returnvalue_x _returnvalue_y) (`KismetMathLibrary.BreakVector` (`self.GetActorScale3D`)))
  (bind _meshlength (`self.meshLength`))
  (set `self.meshLength` (* 45.0 _returnvalue_y))
  (for _index (range (+ (`KismetMathLibrary.FTrunc` (/ (`SplineComponent.GetSplineLength` CurrentSpline) _meshlength)) 1))
    (bind _returnvalue (`AddComponent|NODE_AddSplineMeshComponent-0`))
    (`SplineMeshComponent.SetForwardAxis` _returnvalue "Y" true)
    (`PrimitiveComponent.SetCollisionEnabled` _returnvalue "QueryAndProbe")
    (bind _returnvalue_2 (* _meshlength _index))
    (bind _returnvalue_3 (* (+ _index 1) _meshlength))
    (`SplineMeshComponent.SetStartAndEnd` _returnvalue (`SplineComponent.GetLocationAtDistanceAlongSpline` CurrentSpline _returnvalue_2 "Local") (`KismetMathLibrary.ClampVectorSize` (`SplineComponent.GetTangentAtDistanceAlongSpline` CurrentSpline _returnvalue_2 "Local") 0.0 (`self.meshLength`)) (`SplineComponent.GetLocationAtDistanceAlongSpline` CurrentSpline _returnvalue_3 "Local") (`KismetMathLibrary.ClampVectorSize` (`SplineComponent.GetTangentAtDistanceAlongSpline` CurrentSpline _returnvalue_3 "Local") 0.0 (`self.meshLength`)) true)
    (return)))

(fn `UserConstructionScript`
  (bind (_returnvalue_x _returnvalue_y) (`KismetMathLibrary.BreakVector` (`self.GetActorScale3D`)))
  (bind _spline (`self.Spline`))
  (bind _meshlength (`self.meshLength`))
  (set `self.meshLength` (* 45.0 _returnvalue_y))
  (for _index (range (+ (`KismetMathLibrary.FTrunc` (/ (`SplineComponent.GetSplineLength` _spline) _meshlength)) 1))
    (bind _returnvalue (`AddComponent|NODE_AddSplineMeshComponent-1`))
    (`SplineMeshComponent.SetForwardAxis` _returnvalue "Y" true)
    (`PrimitiveComponent.SetCollisionEnabled` _returnvalue "QueryAndProbe")
    (bind _returnvalue_2 (* _meshlength _index))
    (bind _returnvalue_3 (* (+ _index 1) _meshlength))
    (`SplineMeshComponent.SetStartAndEnd` _returnvalue (`SplineComponent.GetLocationAtDistanceAlongSpline` _spline _returnvalue_2 "Local") (`KismetMathLibrary.ClampVectorSize` (`SplineComponent.GetTangentAtDistanceAlongSpline` _spline _returnvalue_2 "Local") 0.0 (`self.meshLength`)) (`SplineComponent.GetLocationAtDistanceAlongSpline` _spline _returnvalue_3 "Local") (`KismetMathLibrary.ClampVectorSize` (`SplineComponent.GetTangentAtDistanceAlongSpline` _spline _returnvalue_3 "Local") 0.0 (`self.meshLength`)) true)))