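; BP_Projectile is a quark pickup that the player collects by interacting with it.
; Construction applies the base Niagara system to QuarkBody, and BeginPlay starts QuarkLp when IsQuark is set.
; Interact gives the quark to the character, stops it blocking Visibility, swaps to the equipped system, then, if the UI is valid, shows a congrats prompt and broadcasts QuarkObtained.
; ActivateQuark is an empty function taking press state and a skeletal mesh.
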(event `self.ReceiveBeginPlay`
  (`parent.ReceiveBeginPlay`)
  (if (`self.IsQuark`)
    (`AudioComponent.Play` (`self.QuarkLp`) 0.0)))

(event `/Game/Blueprints/Interfaces/Interactable.Interact`
  (params (Character :type "/Game/Blueprints/BP_PlayerCharacter Object Reference") (Component :type "PrimitiveComponent Object Reference"))
  (bind _equipped_quark_system (`self.Equipped Quark System`))
  (`/Game/Blueprints/BP_PlayerCharacter.ObtainQuark` Character self)
  (`PrimitiveComponent.SetCollisionResponseToChannel` (`self.Sphere`) "ECC_Visibility" "ECR_Ignore")
  (`/Engine/EditorBlueprintResources/StandardMacros.IsValid` _equipped_quark_system
    (:`Is Valid`
      (`NiagaraComponent.SetAsset` (`self.Quark Body`) _equipped_quark_system true)
      (bind _ui_base (`self.UI Base`)
        (:`then`
          (`/Game/UI/Widgets/W_CUI_Base.PushCongratsPrompt` _ui_base (`self.PuText`) null (`|ConvertAsset` _ui_base) 0)
          (`self.QuarkObtained`))
        (:`else`)))))

(fn `Activate Quark`
  (params (Pressed :type Boolean) (`Skeletal Mesh` :type "SkeletalMeshComponent Object Reference")))

(fn `UserConstructionScript`
  (bind _base_quark_system (`self.Base Quark System`))
  (`/Engine/EditorBlueprintResources/StandardMacros.IsValid` _base_quark_system
    (:`Is Valid`
      (`NiagaraComponent.SetAsset` (`self.Quark Body`) _base_quark_system true))))