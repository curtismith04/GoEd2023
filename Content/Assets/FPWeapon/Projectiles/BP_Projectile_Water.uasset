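; Water spray "Quark" for the first-person weapon that pushes physics objects, extinguishes burning ones and triggers water-reactive actors.
; BeginPlay attaches an inactive Niagara spray to the QuarkBody; ActivateQuark toggles it, a sound and a looping trace timer with the press state.
; Rather than moving a projectile, WaterTrace repeatedly line-traces from the gun muzzle.
; Component tags route each hit: Immune blocks impulses, Burning calls Extinguish, Water calls WaterEvent.
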(event `self.ReceiveBeginPlay`
  (`parent.ReceiveBeginPlay`)
  (bind _returnvalue (`NiagaraFunctionLibrary.SpawnSystemAttached` "/Game/VFXs/NS_WaterSpray.NS_WaterSpray" (`self.Quark Body`) "None" (100.0 0.0 0.0) (struct) "SnapToTarget" false false))
  (set `self.System` _returnvalue))

(fn `Activate Quark`
  (params (Pressed :type Boolean) (`Skeletal Mesh` :type "SkeletalMeshComponent Object Reference"))
  (bind _quarklp (`self.QuarkLp`))
  (if Pressed
    (set `self.Gun Mesh` `Skeletal Mesh`)
    (bind _returnvalue (`KismetSystemLibrary.K2_SetTimer` null "WaterTrace" 0.05 true))
    (set `self.WaterHandle` _returnvalue)
    (`ActorComponent.Activate` (`self.System`) false)
    (`AudioComponent.Play` (`self.QuarkLp`) 0.0)
    (else
      (`KismetSystemLibrary.K2_ClearAndInvalidateTimerHandle` (`self.WaterHandle`))
      (`ActorComponent.Deactivate` (`self.System`))
      (`AudioParameterControllerInterface.SetTriggerParameter` _quarklp "Stop")
      (`AudioComponent.FadeOut` _quarklp 0.1 0.0 "Linear"))))

(fn `UserConstructionScript`
  (`parent.UserConstructionScript`))

(fn `WaterTrace`
  (bind _gun_mesh (`self.Gun Mesh`))
  (bind _returnvalue (`SceneComponent.GetSocketLocation` _gun_mesh "Muzzle"))
  (bind (_outhit _returnvalue_2) (`KismetSystemLibrary.LineTraceSingle` :`Start` _returnvalue :`End` (+ _returnvalue (* (`SceneComponent.GetForwardVector` (`SceneComponent.GetAttachParent` _gun_mesh)) (`self.Trace Distance`))) :`TraceChannel` "TraceTypeQuery1" :`TraceColor` (struct :`G` 0.25532 :`B` 1.0 :`A` 1.0) :`TraceHitColor` (struct :`G` 1.0 :`B` 0.982993 :`A` 1.0) :`DrawTime` 1.0))
  (if _returnvalue_2
    (`|ExecutionSequence`
      (:`then_0`
        (bind (_bblockinghit _binitialoverlap _time _distance _location _impactpoint _normal _impactnormal _physmat _hitactor _hitcomponent _hitbonename _bonename _hititem _elementindex _faceindex _tracestart _traceend) (`GameplayStatics.BreakHitResult` _outhit))
        (if (and (`SceneComponent.IsSimulatingPhysics` _hitcomponent "None") (not (`ActorComponent.ComponentHasTag` _hitcomponent "Immune")))
          (`PrimitiveComponent.AddVelocityChangeImpulseAtLocation` _hitcomponent (* (`KismetMathLibrary.Normal` (- _tracestart _traceend)) -10.0) _impactpoint "None")))
      (:`then_1`
        (if (`ActorComponent.ComponentHasTag` _hitcomponent "Burning")
          (`/Game/Blueprints/Interfaces/Burnable.Extinguish` (cast `/Game/Blueprints/Interfaces/Burnable` _hitactor :!pure true))))
      (:`then_2`
        (if (`ActorComponent.ComponentHasTag` _hitcomponent "Water")
          (`/Game/Blueprints/Interfaces/Water.Water Event` (cast `/Game/Blueprints/Interfaces/Water` _hitactor :!pure true) _hitcomponent _outhit))))))