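; Gravity "quark" for the first-person weapon that toggles gravity on the actor it hits.
; On press, ActivateQuark attaches a Niagara arc beam to QuarkBody, triggers the QuarkLp "Fire" parameter and runs a visibility line trace from the Muzzle socket along the mesh parent's forward vector.
; The trace sets beam length from hit or maximum distance and flips gravity through the target's AC_GravityComponent, if present.
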(fn `Activate Quark`
  (params (Pressed :type Boolean) (`Skeletal Mesh` :type "SkeletalMeshComponent Object Reference"))
  (if Pressed
    (bind _returnvalue (`NiagaraFunctionLibrary.SpawnSystemAttached` "/Game/VFXs/Weapon_VFX/GravityGun_VFX/NS_GravityArcs.NS_GravityArcs" (`self.Quark Body`) "None" (0.0 0.0 0.0) (struct) "KeepRelativeOffset"))
    (set `self.Beam` _returnvalue)
    (`AudioParameterControllerInterface.SetTriggerParameter` (`self.QuarkLp`) "Fire")
    (bind (_returnvalue_2 _outhit) (`self.Line Trace` `Skeletal Mesh`))
    (if _returnvalue_2
      (bind (_bblockinghit _binitialoverlap _time _distance _location _impactpoint _normal _impactnormal _physmat _hitactor) (`GameplayStatics.BreakHitResult` _outhit))
      (`FXSystemComponent.SetVectorParameter` (`self.Beam`) "User.BeamEnd" (`KismetMathLibrary.MakeVector` _distance))
      (bind _returnvalue_3 (`self.GetComponentByClass` _hitactor "/Game/Blueprints/Components/AC_GravityComponent.AC_GravityComponent_C"))
      (`/Engine/EditorBlueprintResources/StandardMacros.IsValid` _returnvalue_3
        (:`Is Valid`
          (`/Game/Blueprints/Components/AC_GravityComponent.Toggle Gravity` _returnvalue_3 (not (`/Game/Blueprints/Components/AC_GravityComponent.isGravityOn` _returnvalue_3)))))
      (else
        (`FXSystemComponent.SetVectorParameter` (`self.Beam`) "User.BeamEnd" (`KismetMathLibrary.MakeVector` (`self.Trace Distance`)))))))

(fn `UserConstructionScript`
  (`parent.UserConstructionScript`))