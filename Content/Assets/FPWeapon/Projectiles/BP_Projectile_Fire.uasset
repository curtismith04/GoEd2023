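; BP_Projectile_Fire is a fire weapon "Quark" that launches BP_Fireball projectiles when activated.
; On press, ActivateQuark spawns a fireball just ahead of the supplied mesh's Muzzle socket, passing the attach parent's forward vector as its velocity, and plays a firing sound.
; A CanFire flag and a FireRate timer calling Reset limit it to one shot per press and interval, with no automatic repeat.
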(fn `Activate Quark`
  (params (Pressed :type Boolean) (`Skeletal Mesh` :type "SkeletalMeshComponent Object Reference"))
  (bind _returnvalue (`SceneComponent.GetForwardVector` (`SceneComponent.GetAttachParent` `Skeletal Mesh`)))
  (if Pressed
    (if (`self.CanFire`)
      (`|SpawnActorFromClass` "/Game/Blueprints/BP_Fireball.BP_Fireball_C" (`KismetMathLibrary.MakeTransform` (+ (`SceneComponent.GetSocketLocation` `Skeletal Mesh` "Muzzle") (* _returnvalue 100.0))) "AlwaysSpawn" "MultiplyWithRoot" null _returnvalue null)
      (set `self.CanFire` false)
      (bind _returnvalue_2 (`KismetSystemLibrary.K2_SetTimer` null "Reset" (`self.FireRate`)))
      (set `self.FireHandle` _returnvalue_2)
      (`GameplayStatics.PlaySound2D` "/Game/Audio/SFX/SFX_Plyr_FireGun.SFX_Plyr_FireGun" 1.0 1.0 0.0 null null))))

(fn `Reset`
  (set `self.CanFire` true)
  (`KismetSystemLibrary.K2_ClearAndInvalidateTimerHandle` (`self.FireHandle`)))

(fn `UserConstructionScript`
  (`parent.UserConstructionScript`))